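; GA_Test is a test gameplay ability that fires a projectile from its avatar.
; After committing, it line-traces forward on Visibility over the weapon range.
; On a hit, it spawns a Niagara effect at the impact and a BP_AtomProjectile ahead of the avatar, facing forward.
; It ends only when the commit fails; hit-notify and force-field spawn nodes are left disconnected.
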(event `self.K2_ActivateAbility`
  (bind (_owneractor _avataractor) (break `GameplayAbilityActorInfo` (`self.GetActorInfo`)))
  (bind _returnvalue (`Actor.K2_GetActorLocation` _avataractor))
  (bind _returnvalue_2 (`Actor.GetActorForwardVector` _avataractor))
  (bind _returnvalue_3 (`self.K2_CommitAbility`))
  (if _returnvalue_3
    (set `self.Location` _returnvalue)
    (set `self.Direction` _returnvalue_2)
    (bind (_outhit _returnvalue_4) (`KismetSystemLibrary.LineTraceSingle` _returnvalue (+ _returnvalue (* _returnvalue_2 (`self.WeaponRange`))) "TraceTypeQuery1"))
    (`|ExecutionSequence`
      (:`then_1`
        (if _returnvalue_4
          ;[1 1 1] Effect
          (`NiagaraFunctionLibrary.SpawnSystemAtLocation` "/Game/AbilitySystem/NewNiagaraSystem.NewNiagaraSystem" (`.Location` (`GameplayStatics.BreakHitResult` _outhit)) (struct) (1.0 1.0 1.0) true true "AutoRelease")
          (`|SpawnActorFromClass` "/Game/Chaos/BP_AtomProjectile.BP_AtomProjectile_C" (`KismetMathLibrary.MakeTransform` (+ (`self.Location`) (* (`self.Direction`) (`self.Distance`))) (`KismetMathLibrary.FindLookAtRotation` (`KismetMathLibrary.Vector_Zero`) (`self.Direction`))) "Undefined" "MultiplyWithRoot" null null))))
    (else
      (`self.K2_EndAbility`))))