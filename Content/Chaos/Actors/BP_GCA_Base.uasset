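; Base Chaos geometry collection actor that gets an inverse-gravity force until it breaks, then destroys itself after a delay.
; Tick applies a vertical force scaled from world gravity and ForceMultiplier until the Chaos break event cancels it.
; The construction script creates dynamic instances of its first three materials.
; BP_Controller's suspend and resume events play or reverse a timeline driving those materials' Hide parameter.
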(event `self.ReceiveBeginPlay`
  (bind _asbp_controller (cast `/Game/Core/BP_Controller` (`GameplayStatics.GetPlayerController` 0)))
  (add `CubeizationPlayerController.OnSuspend` _asbp_controller (delegate `On Suspend`))
  (add `CubeizationPlayerController.OnResume` _asbp_controller (delegate `On Resume`)))

(event `On Suspend`
  (bind (_direction _hide) (`Timeline|Timeline` :!label _label)
    (:`Update`
      (`MaterialInstanceDynamic.SetScalarParameterValue` (`self.Mat1`) "Hide" _hide)
      (`MaterialInstanceDynamic.SetScalarParameterValue` (`self.Mat2`) "Hide" _hide)
      (`MaterialInstanceDynamic.SetScalarParameterValue` (`self.Mat3`) "Hide" _hide))))

(event `On Resume`
  (goto _label :!via `Reverse`))

(event `self.ReceiveTick`
  (params (DeltaSeconds :type "Float (single-precision)"))
  (`|ExecutionSequence`
    (:`then_0`
      (if (not (`self.CancelInverseGravity`))
        (bind _gravityz (`BlueprintUtils.GetWorldGravityZ` self))
        (bind _result (`/Engine/EditorBlueprintResources/StandardMacros.NegateFloat` (* _gravityz (`self.ForceMultiplier`)))
          (:`  `
            (`PrimitiveComponent.AddForce` (`self.GeometryCollectionComponent`) (`KismetMathLibrary.MakeVector` 0.0 0.0 _result) "None" false)))))))

(event `self.GeometryCollectionComponent.OnChaosBreakEvent`
  (params (BreakEvent :type "ChaosBreakEvent Structure (by ref)"))
  (set `self.CancelInverseGravity` true)
  (`KismetSystemLibrary.Delay` 25.0)
  (`self.K2_DestroyActor`))

(fn `UserConstructionScript`
  (bind _geometrycollectioncomponent (`self.GeometryCollectionComponent`))
  (for (_array_element _array_index) (`MeshComponent.GetMaterials` (`self.GeometryCollectionComponent`))
    (switch `int` _array_index
      (:`0`
        (bind _returnvalue (`PrimitiveComponent.CreateDynamicMaterialInstance` _geometrycollectioncomponent _array_index _array_element "None"))
        (set `self.Mat1` _returnvalue))
      (:`1`
        (bind _returnvalue_2 (`PrimitiveComponent.CreateDynamicMaterialInstance` _geometrycollectioncomponent _array_index _array_element "None"))
        (set `self.Mat2` _returnvalue_2))
      (:`2`
        (bind _returnvalue_3 (`PrimitiveComponent.CreateDynamicMaterialInstance` _geometrycollectioncomponent _array_index _array_element "None"))
        (set `self.Mat3` _returnvalue_3)))))